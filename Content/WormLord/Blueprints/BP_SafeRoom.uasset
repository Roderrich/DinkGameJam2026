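; BP_SafeRoom is a room that can host an emergency disturbance (police, electrician, cleaner or fire department) and reports a point score.
; Activation with the annoy flag starts the chosen disturbance and a looping timer that restores points once solved, or zeroes them after repeated unsolved loops.
; NoiseActivated adds points gathered from annoying worms to the room's total.
; The four per-disturbance functions are empty stubs, and activation and deactivation print debug text.
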(event Custom|ActivateEvent
  (Variables|Default|SetIsActive true)
  (bind _returnvalue (Utilities|Time|SetTimerbyEvent (delegate Custom|StartOfDistrubance) (Variables|Default|GetActiveDuration) true))
  (Variables|Default|SetTimerRef _returnvalue))

(event Custom|StartOfDistrubance
  (if (Variables|Default|GetSolved?)
    (Variables|Default|SetIsActive false)
    (Variables|Default|SetSolved? false)
    (Utilities|Time|ClearandInvalidateTimerbyHandle (Variables|Default|GetTimerRef))
    (Variables|Default|SetCurrentPoints 2)
    (else
      (bind _result (Math|Integer|IncrementInt (Variables|Default|GetAmountOfLoops))
        (:%20%20
          (if (>= _result 3)
            (Variables|Default|SetCurrentPoints 0)))))))

(event Custom|StartEvent
  (params (Int :type E_EmergancyServices%20Enum :default "NewEnumerator0"))
  (Variables|Default|SetCurrentPoints 1)
  (bind _output_get (Variables|Default|SetCurrentDisturbance Int))
  (switch Utilities|FlowControl|Switch|SwitchonE_EmergancyServices _output_get
    (:NewEnumerator0
      (CallFunction|Disturbance1))
    (:NewEnumerator1
      (CallFunction|Disturbance2))
    (:NewEnumerator2
      (CallFunction|Disturbance3))
    (:NewEnumerator3
      (CallFunction|Disturbance4))))

(event EventBeginPlay)

(event EventActivated
  (params (Annoy :type Boolean) (Enum :type E_EmergancyServices%20Enum :default "NewEnumerator0"))
  (Variables|Default|SetIsActive true)
  (if Annoy
    (CallFunction|StartEvent Enum)
    (CallFunction|ActivateEvent)
    (Development|PrintString (Utilities|String|ToString(Text) (Utilities|Text|FormatText "room: {Q} 
Emergancy:{B}" (Variables|Default|GetRoom) (|GenerictoText (Variables|Default|GetCurrentDisturbance)))))))

(event EventDeactivated
  (Variables|Default|SetIsActive false)
  (Development|PrintString (Utilities|String|ToString(Text) (Utilities|Text|FormatText "Room: {Q} Deactivated" (Variables|Default|GetRoom))) true true "(R=0.000000,G=0.660000,B=1.000000,A=1.000000)" 1e+01)
  (Variables|Default|SetCurrentPoints 2)
  (Variables|Default|SetAmountOfLoops 0))

(event EventNoiseActivated
  (for _array_element (Variables|Default|GetAnnoyingWorms)
    (bind _points (Class|BPIRooms|GetPoints(Message) _array_element))
    (Variables|Default|SetAnnoyRoomPoints (+ _points (Variables|Default|GetAnnoyRoomPoints)))))

(fn ConstructionScript)

(fn Disturbance1)

(fn Disturbance2)

(fn Disturbance3)

(fn Disturbance4)

(fn CheckActive
  (return (Variables|Default|GetIsActive)))

(fn SetSolved
  (params (Solved? :type Boolean))
  (Variables|Default|SetSolved? Solved?))

(fn GetActive
  (return (Variables|Default|GetIsActive)))

(fn GetPoints
  (return (+ (Variables|Default|GetCurrentPoints) (Variables|Default|GetAnnoyRoomPoints))))

(fn GetRoomNumber
  (return (Variables|Default|GetRoom)))

(fn TypeOfEvent
  (return (Variables|Default|GetCurrentDisturbance)))