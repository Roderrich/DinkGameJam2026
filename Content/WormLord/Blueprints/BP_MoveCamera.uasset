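; BP_MoveCamera is a trigger volume that moves the player's camera to a locked viewpoint and activates its linked doors.
; Box overlap by the third-person character sends MoveCameraMessage with an offset from the actor's root, activates the Doors array and starts mouse tracking.
; The Back event sends the camera to a second offset, deactivates the doors and stops tracking.
; SetTheDoor stores the door interacted with.
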(event OnComponentBeginOverlap(Box)
  (params (OverlappedComponent :type Primitive%20Component%20Object%20Reference) (OtherActor :type Actor%20Object%20Reference) (OtherComp :type Primitive%20Component%20Object%20Reference) (OtherBodyIndex :type Integer) (bFromSweep :type Boolean) (SweepResult :type Hit%20Result%20Structure%20%28by%20ref%29))
  (bind _asbp_third_person_character (Utilities|Casting|CastToBP_ThirdPersonCharacter OtherActor))
  (Class|BPIPlayer|MoveCamera(Message) _asbp_third_person_character (+ (Transformation|GetWorldLocation (Variables|Default|GetDefaultSceneRoot)) (Variables|Default|GetCameraLocation)) (Variables|Default|GetRight) true self)
  (for _array_element (Variables|Default|GetDoors)
    (Default|SetActivated _array_element true))
  (Default|StartTrackingMouse (Variables|Default|GetPlayerRef)))

(event Custom|SetTheDoor
  (params (Door :type Actor%20Object%20Reference))
  (Variables|Default|SetDoorInteractedWith Door))

(event EventBeginPlay
  (bind _asbp_third_person_character (Utilities|Casting|CastToBP_ThirdPersonCharacter (Game|GetPlayerCharacter 0)))
  (Variables|Default|SetPlayerRef _asbp_third_person_character))

(event Collision|EventActorBeginOverlap
  (params (OtherActor :type Actor%20Object%20Reference)))

(event EventTick
  (params (DeltaSeconds :type Float%20%28single-precision%29)))

(event EventBack
  (bind _asbp_third_person_character (Utilities|Casting|CastToBP_ThirdPersonCharacter (Game|GetPlayerCharacter 0)))
  (Class|BPIPlayer|MoveCamera(Message) _asbp_third_person_character (+ (Transformation|GetWorldLocation (Variables|Default|GetDefaultSceneRoot)) (Variables|Default|GetCameraLocation2)) false false self)
  (for _array_element (Variables|Default|GetDoors)
    (Default|SetActivated _array_element false))
  (Default|StopTrackingMouse (Variables|Default|GetPlayerRef)))

(fn ConstructionScript)