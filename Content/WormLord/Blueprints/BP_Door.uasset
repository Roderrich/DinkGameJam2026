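; BP_Door is a clickable door that responds to clicks only while activated.
; An external SetActivated event toggles its IsActivated flag, and BeginPlay binds a handler to the actor's OnClicked event.
; A click on an active door passes the touched actor to MoveCamera as the door and calls DeactivatedMessage on its RoomReference.
; A disconnected branch querying the room's event message type never runs.
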(event Custom|SetActivated
  (params (IsActivated :type Boolean))
  (Variables|Default|SetIsActivated IsActivated))

(event Custom|OnClicked_Event
  (params (TouchedActor :type Actor%20Object%20Reference) (ButtonPressed :type Key%20Structure :default "None"))
  (if (Variables|Default|GetIsActivated)
    (Default|SettheDoor (Variables|Default|GetMoveCamera) TouchedActor)
    (Class|BPIRooms|Deactivated(Message) (Variables|Default|GetRoomReference))))

(event EventBeginPlay
  (EventDispatchers|BindEventtoOnClicked (delegate Custom|OnClicked_Event)))

(fn ConstructionScript)