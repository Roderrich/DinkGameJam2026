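; BP_AnnoyRoom is a numbered room that can host either a noise annoyance or an emergency disturbance, exposing its active state, event type and points.
; Activation sets points by event type and starts a looping timer that clears once solved, or worsens the penalty after repeated unsolved loops.
; Deactivating an active room awards a point, without clearing the timer.
; The numbered Disturbance and Noise functions are empty stubs, and state changes print debug strings.
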(event Custom|ActivateEvent
  (Variables|Default|SetIsActive true)
  (bind _returnvalue (Utilities|Time|SetTimerbyEvent (delegate Custom|StartOfDistrubance) (Variables|Default|GetActiveDuration) true))
  (Variables|Default|SetEventLoop _returnvalue))

(event Custom|StartOfDistrubance
  (if (Variables|Default|GetSolved?)
    (Variables|Default|SetSolved? false)
    (Variables|Default|SetIsActive false)
    (Utilities|Time|ClearandInvalidateTimerbyHandle (Variables|Default|GetEventLoop))
    (else
      (bind _result (Math|Integer|IncrementInt (Variables|Default|GetAmountOfLoops))
        (:%20%20
          (if (>= _result 3)
            (Variables|Default|SetCurrentPoints -2)))))))

(event Custom|StartDisturbance
  (params (Disturbance :type E_EmergancyServices%20Enum :default "NewEnumerator0"))
  (Variables|Default|SetCurrentPoints -1))

(event Custom|StartNoiseEvent
  (params (Int :type Integer))
  (Variables|Default|SetCurrentPoints 0))

(event EventActivated
  (params (Annoy :type Boolean) (Enum :type E_EmergancyServices%20Enum :default "NewEnumerator0"))
  (Variables|Default|SetIsActive true)
  (if Annoy
    (Variables|Default|SetCurrentDisturbance "NewEnumerator4")
    (CallFunction|StartNoiseEvent)
    (Development|PrintString (Utilities|String|ToString(Integer) (Variables|Default|GetRoom)) true true "(R=1.000000,G=0.955231,B=0.970345,A=1.000000)" 5.0)
    (else
      (bind _output_get (Variables|Default|SetCurrentDisturbance Enum))
      (CallFunction|StartDisturbance _output_get)
      (Development|PrintString (Utilities|String|ToString(Text) (Utilities|Text|FormatText "room: {Q} 
Emergancy:{B}" (Variables|Default|GetRoom) (|GenerictoText (Variables|Default|GetCurrentDisturbance)))))))
  (CallFunction|ActivateEvent))

(event EventDeactivated
  (if (Variables|Default|GetIsActive)
    (Variables|Default|SetIsActive false)
    (Development|PrintString (Utilities|String|ToString(Text) (Utilities|Text|FormatText "Room: {Q} Deactivated" (Variables|Default|GetRoom))) true true "(R=0.000000,G=0.660000,B=1.000000,A=1.000000)" 1e+01)
    (Variables|Default|SetCurrentPoints 1)))

(event EventBeginPlay)

(fn ConstructionScript)

(fn CheckActive
  (return (Variables|Default|GetIsActive)))

(fn SetSolved
  (params (Solved? :type Boolean))
  (Variables|Default|SetSolved? Solved?))

(fn Disturbance1)

(fn Disturbance2)

(fn Disturbance3)

(fn Disturbance4)

(fn Noise1)

(fn Noise2)

(fn Noise3)

(fn Noise4
  (return))

(fn GetActive
  (return (Variables|Default|GetIsActive)))

(fn GetPoints
  (return (Variables|Default|GetCurrentPoints)))

(fn GetRoomNumber
  (return (Variables|Default|GetRoom)))

(fn TypeOfEvent
  (return (Variables|Default|GetCurrentDisturbance)))