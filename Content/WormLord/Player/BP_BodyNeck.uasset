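; BP_BodyNeck is an actor that trails a FollowObject, apparently the neck segment of the player's worm body.
; Each Tick, while FollowObject is valid, it interpolates toward a point just behind that object's forward vector.
; Its Z is pinned to a Height variable and its roll is fixed, while yaw is interpolated to face the followed object.
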(event EventBeginPlay)

(event Collision|EventActorBeginOverlap
  (params (OtherActor :type Actor%20Object%20Reference)))

(event EventTick
  (params (DeltaSeconds :type Float%20%28single-precision%29))
  (bind _returnvalue (Transformation|GetActorLocation))
  (bind _followobject (Variables|Default|GetFollowObject))
  (bind _returnvalue_2 (Transformation|GetActorLocation _followobject))
  (bind _returnvalue_3 (Transformation|GetActorForwardVector _followobject))
  (bind _returnvalue_4 (* _returnvalue_3 1e+01))
  (bind _returnvalue_5 (- _returnvalue_2 _returnvalue_4))
  (bind _returnvalue_6 (Math|Interpolation|VInterpTo _returnvalue _returnvalue_5 DeltaSeconds 25.0))
  (Utilities|IsValid (Variables|Default|GetFollowObject)
    (:Is%20Valid
      (Transformation|SetActorLocationAndRotation (Math|Vector|MakeVector (.x _returnvalue_6) (.y _returnvalue_6) (Variables|Default|GetHeight)) (Math|Rotator|MakeRotator -9e+01 0.0 (.yaw (Math|Interpolation|RInterpTo (Transformation|GetActorRotation) (Math|Rotator|FindLookatRotation _returnvalue _returnvalue_2) DeltaSeconds 0.0)))))))

(fn ConstructionScript)